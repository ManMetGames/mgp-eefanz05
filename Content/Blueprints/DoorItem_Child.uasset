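; Door item child Blueprint that hands player control to the lockpicking character when interacted with.
; On Interact, it checks the CanPressE and CanInteract flags, then clears CanInteract so the switch happens once.
; It finds the MyLockpick_Character_BP instance in the level and has player controller 0 possess it.
; The construction script only calls the parent's.
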(event `/Game/Blueprints/Interaction.Interact`
  (if (`self.CanPressE`)
    (if (`self.CanInteract`)
      (set `self.CanInteract` false)
      (if true
        (bind _returnvalue (`GameplayStatics.GetActorOfClass` "/Game/Blueprints/MyLockpick_Character_BP.MyLockpick_Character_BP_C"))
        (`Controller.Possess` (`GameplayStatics.GetPlayerController` 0) _returnvalue)))))

(fn `UserConstructionScript`
  (`parent.UserConstructionScript`))